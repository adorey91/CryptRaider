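; BP_KeyItemReset is an actor component, apparently meant to return a moved key item to its starting location when it is not grabbed.
; BeginPlay stores and prints the owner's location, while Tick is empty and the distance and "Grabbed" tag check leading to CountdownEvent is unconnected.
; CountdownEvent prints Countdown minus one frame's delta, without accumulating, then moves the owner back immediately, using timer expiry only as the Sweep flag.
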(event Custom|CountdownEvent
  (bind _output_get (Variables|Default|Settimer (Math|Float|Clamp(Float) (- (Variables|Default|Getcountdown) (Utilities|Time|GetWorldDeltaSeconds)) 0.0 (Variables|Default|Getcountdown))))
  (Development|PrintString (Class|KismetStringLibrary|TimeSecondstoString _output_get))
  (Transformation|SetActorLocation (Components|GetOwner) (Variables|Default|GetstartingLocation) (<= _output_get 0.0) false))

(event EventBeginPlay
  (bind _output_get (Variables|Default|SetstartingLocation (Transformation|GetActorLocation (Components|GetOwner))))
  (Development|PrintString (Utilities|String|ToString(Vector) _output_get)))

(event EventTick
  (params (DeltaSeconds :type Float%20%28single-precision%29)))