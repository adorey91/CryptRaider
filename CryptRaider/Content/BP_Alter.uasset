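; BP_Alter is an actor, apparently a movable stone altar, that plays a stone-pushing sound while it moves.
; Each tick it reads the Mover component's ShouldPlaySFX flag, starting the StonePush audio if it is not already playing and stopping it otherwise.
; The sound is silenced at BeginPlay, and the movement logic itself lives in Mover, outside this graph.
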(event EventBeginPlay
  (Audio|Components|Audio|Stop (Variables|Default|GetStonePush)))

(event Collision|EventActorBeginOverlap
  (params (OtherActor :type Actor%20Object%20Reference)))

(event EventTick
  (params (DeltaSeconds :type Float%20%28single-precision%29))
  (bind _stonepush (Variables|Default|GetStonePush))
  (if (Variables|/Script/CryptRaider.Mover|GetShouldPlaySFX (Variables|Default|GetMover))
    (if (not (Audio|Components|Audio|IsPlaying _stonepush))
      (Audio|Components|Audio|Play _stonepush 0.0))
    (else
      (Audio|Components|Audio|Stop (Variables|Default|GetStonePush)))))

(fn ConstructionScript)