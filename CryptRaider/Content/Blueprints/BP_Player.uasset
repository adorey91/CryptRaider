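; Player Blueprint that handles grabbing objects and detecting interactable actors under the camera's view.
; Grab input starts and releases through a Grabber component, which also provides a highlight check.
; A looping timer sphere-traces WorldDynamic objects from the camera along control rotation.
; Hits implementing BPI_Interactions receive LookAtMessage on or off as the tracked look-at actor changes or the trace misses.
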(event Input|EnhancedActionEvents|EnhancedInputActionIA_Grab
  (params (ActionValue :type Boolean) (ElapsedSeconds :type Float%20%28double-precision%29) (TriggeredSeconds :type Float%20%28double-precision%29) (InputAction :type Input%20Action%20Object%20Reference :default "/Game/FirstPerson/Input/Actions/IA_Grab.IA_Grab"))
  (bind _grabber (Variables|Default|GetGrabber))
  (:Started
    (Class|Grabber|Grab _grabber))
  (:Completed
    (Class|Grabber|Release _grabber)))

(event EventBeginPlay
  (Utilities|Time|SetTimerbyFunctionName 0 "Check Interaction" 0.5 true true))

(event EventTick
  (params (DeltaSeconds :type Float%20%28single-precision%29)))

(fn ConstructionScript
  (|CallParentFunction))

(fn CheckforHighlight
  (Class|Grabber|CheckforHighlight (Variables|Default|GetGrabber)))

(fn CheckInteraction
  (bind _returnvalue (Game|GetPlayerCameraManager 0))
  (bind _returnvalue_2 (Camera|GetCameraLocation _returnvalue))
  (bind (_outhit _returnvalue_3) (Collision|SphereTraceForObjects _returnvalue_2 (+ _returnvalue_2 (* (Math|Vector|GetForwardVector (Pawn|GetControlRotation (Pawn|GetController (Game|Player|GetPlayerPawn 0)) :!class /Script/Engine.Controller)) 1.5e+03)) 1e+02 (Utilities|Array|MakeArray "ObjectTypeQuery2") false 0 "None"))
  (if _returnvalue_3
    (if (Utilities|DoesObjectImplementInterface (.HitActor (Collision|BreakHitResult _outhit)) "/Game/Interfaces/BPI_Interactions.BPI_Interactions_C")
      (Variables|Default|SetLookAtActor_Current (.HitActor (Collision|BreakHitResult _outhit)))
      (Utilities|IsValid (Variables|Default|GetLookAtActor_Old)
        (:Is%20Valid
          (if (== (Variables|Default|GetLookAtActor_Current) (Variables|Default|GetLookAtActor_Old))
            (Class|BPIInteractions|Lookat(Message) (Variables|Default|GetLookAtActor_Old) true)
            (Variables|Default|SetLookingAt false)
            (else
              (Class|BPIInteractions|Lookat(Message) (Variables|Default|GetLookAtActor_Old) false)
              (Variables|Default|SetLookAtActor_Old (Variables|Default|GetLookAtActor_Current) :!label _label)
              (Class|BPIInteractions|Lookat(Message) (Variables|Default|GetLookAtActor_Current) true)
              (Variables|Default|SetLookingAt false))))
        (:Is%20Not%20Valid
          (goto _label))))
    (else
      (Utilities|IsValid (Variables|Default|GetLookAtActor_Old)
        (:Is%20Valid
          (Class|BPIInteractions|Lookat(Message) (Variables|Default|GetLookAtActor_Old) false))
        (:Is%20Not%20Valid
          _))
      (Variables|Default|SetLookingAt false))))