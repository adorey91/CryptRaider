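; BP_SecretWall is a secret wall actor that pairs a Trigger component with a Mover component and a stone-pushing sound.
; At begin play it hands the Mover to the Trigger and stops the StonePush audio.
; The Mover's play-sound and stop-sound events start and stop StonePush, so the audio follows the Mover's own signals.
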(event OnPlaySound(Mover)
  (Audio|Components|Audio|Play (Variables|Default|GetStonePush) 0.0))

(event OnStopSound(Mover)
  (Audio|Components|Audio|Stop (Variables|Default|GetStonePush)))

(event EventBeginPlay
  (Class|TriggerComponent|SetMover (Variables|Default|GetTrigger) (Variables|Default|GetMover))
  (Audio|Components|Audio|Stop (Variables|Default|GetStonePush)))

(event Collision|EventActorBeginOverlap
  (params (OtherActor :type Actor%20Object%20Reference)))

(event EventTick
  (params (DeltaSeconds :type Float%20%28single-precision%29)))

(fn ConstructionScript)