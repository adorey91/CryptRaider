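; BP_Coffin is a coffin actor that tracks the weight of physics objects inside its Trigger.
; On BeginPlay it records the starting weight as the Trigger's WeightNeeded, then starts a delayed looping timer that re-measures.
; Each check sums the mass of simulating StaticMeshActors overlapping the Trigger into CurrentWeight, leaving any reaction to weight changes outside this graph.
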(event EventBeginPlay
  (Utilities|FlowControl|Sequence
    (:then_0
      (bind _output_get (CallFunction|ChecksCurrentWeight))
      (Variables|/Script/CryptRaider.TriggerComponent|SetWeightNeeded (Variables|Default|GetTrigger) _output_get))
    (:then_1
      (bind _returnvalue (Utilities|Time|SetTimerbyFunctionName 0 "CheckWeight" 1.0 true true 3e+01))
      (Variables|Default|SetCheckWeightTimer _returnvalue))))

(event Collision|EventActorBeginOverlap
  (params (OtherActor :type Actor%20Object%20Reference)))

(event EventTick
  (params (DeltaSeconds :type Float%20%28single-precision%29)))

(fn ConstructionScript)

(fn CheckWeight
  (CallFunction|ChecksCurrentWeight))

(fn ChecksCurrentWeight
  (bind _output_get (Variables|Default|SetActor (Collision|GetOverlappingActors (Variables|Default|GetTrigger) "/Script/Engine.StaticMeshActor" :!class /Script/Engine.PrimitiveComponent)))
  (Variables|/Script/CryptRaider.TriggerComponent|SetCurrentWeight (Variables|Default|GetTrigger) 0.0)
  (for _array_element _output_get
    (bind _output_get_2 (Variables|Default|SetMeshComp (Actor|GetComponentbyClass _array_element "/Script/Engine.StaticMeshComponent")))
    (if (Physics|IsSimulatingPhysics _output_get_2 "None")
      (Variables|/Script/CryptRaider.TriggerComponent|SetCurrentWeight (Variables|Default|GetTrigger) (+ (Variables|/Script/CryptRaider.TriggerComponent|GetCurrentWeight (Variables|Default|GetTrigger)) (Physics|GetMass (Variables|Default|GetMeshComp))))))
  (return (Variables|/Script/CryptRaider.TriggerComponent|GetCurrentWeight (Variables|Default|GetTrigger))))