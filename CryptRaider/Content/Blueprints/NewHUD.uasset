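; HUD Blueprint that shows and hides an on-screen current-weight readout using the WP_CurrentWeight widget.
; ShowCurrentWeight creates the widget and adds it to the viewport on a non-zero weight when inactive, then passes it the value.
; While IsActive is set, further calls only update that widget, including with zero.
; HideCurrentWeight removes the widget and clears the flag, so the next non-zero show builds a new instance.
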(event Custom|ShowCurrentWeight
  (params (Current%20Weight :type Float%20%28double-precision%29))
  (if (Variables|Default|GetisActive)
    (bind _output_get (Variables|Default|SetUI_Ref (Variables|Default|GetUI_Ref) :!label _label))
    (Default|CurrentWeight _output_get Current%20Weight)
    (elif (!= Current%20Weight 0.0)
      (bind _returnvalue (UserInterface|CreateWidget "/Game/UI/WP_CurrentWeight.WP_CurrentWeight_C"))
      (bind _output_get_2 (Variables|Default|SetUI_Ref _returnvalue))
      (UserInterface|Viewport|AddtoViewport _output_get_2 0)
      (Variables|Default|SetisActive true)
      (goto _label))))

(event Custom|HideCurrentWeight
  (Utilities|IsValid (Variables|Default|GetUI_Ref)
    (:Is%20Valid
      (Widget|RemovefromParent (Variables|Default|GetUI_Ref))
      (Variables|Default|SetisActive false))))

(event EventBeginPlay)

(event Collision|EventActorBeginOverlap
  (params (OtherActor :type Actor%20Object%20Reference)))

(event EventTick
  (params (DeltaSeconds :type Float%20%28single-precision%29)))

(fn ConstructionScript)