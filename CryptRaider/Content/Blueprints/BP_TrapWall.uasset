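; BP_TrapWall is a trap wall actor that plays a JailDoor sound in response to its Mover component.
; Mover's OnPlaySound and OnStopSound events start and stop JailDoor, each checking IsPlaying first so the sound is not restarted or stopped redundantly.
; BeginPlay stops JailDoor so the wall starts silent.
; The Blueprint holds no movement, overlap or tick logic of its own.
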(event OnPlaySound(Mover)
  (if (not (Audio|Components|Audio|IsPlaying (Variables|Default|GetJailDoor)))
    (Audio|Components|Audio|Play (Variables|Default|GetJailDoor) 0.0)))

(event OnStopSound(Mover)
  (if (Audio|Components|Audio|IsPlaying (Variables|Default|GetJailDoor))
    (Audio|Components|Audio|Stop (Variables|Default|GetJailDoor))))

(event EventBeginPlay
  (Audio|Components|Audio|Stop (Variables|Default|GetJailDoor)))

(event Collision|EventActorBeginOverlap
  (params (OtherActor :type Actor%20Object%20Reference)))

(event EventTick
  (params (DeltaSeconds :type Float%20%28single-precision%29)))

(fn ConstructionScript)